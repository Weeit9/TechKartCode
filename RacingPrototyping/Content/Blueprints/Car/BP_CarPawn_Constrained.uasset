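; Physics-driven car pawn with raycast suspension, drifting and a random item slot whose use logic is still a stub.
; Each tick, four corner traces feed suspension components that push the body along ground normals and place wheel meshes.
; Tick also applies lateral grip unless drifting, clamps pitch and roll, and adds downforce when airborne.
; Input drives throttle and steering through local forces, with steering also shifting center of mass and yawing front wheels.
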(event `On Ground Check`
  (if (not (`self.onGround`))
    (`PrimitiveComponent.AddForce` (`self.carBody`) (0.0 0.0 -200000.0) "None" false)))

(event `self.ReceiveTick`
  (params (DeltaSeconds :type "Float (single-precision)"))
  (`self.FD_Thruster`)
  (`self.FP_Thruster`)
  (`self.RD_Thruster`)
  (`self.RP_Thruster`)
  (`self.Grip Handler`)
  (`self.Clamp Rotation`)
  (`self.On Ground Check`))

(event `EnhancedInput|/Game/Data/Input/IA_Drift`
  (params (ActionValue :type Boolean) (ElapsedSeconds :type "Float (double-precision)") (TriggeredSeconds :type "Float (double-precision)") (InputAction :type "InputAction Object Reference" :default "/Game/Data/Input/IA_Drift.IA_Drift"))
  (:`Triggered`
    (set `self.Drifting` true))
  (:`Canceled`
    (set `self.Drifting` false :!label _label))
  (:`Completed`
    (goto _label)))

(event `Clamp Rotation`
  (bind _carbody (`self.carBody`))
  (bind (_returnvalue_roll _returnvalue_pitch _returnvalue_yaw) (`KismetMathLibrary.BreakRotator` (`SceneComponent.K2_GetComponentRotation` _carbody)))
  (`SceneComponent.K2_SetWorldRotation` _carbody (`KismetMathLibrary.MakeRotator` (`KismetMathLibrary.ClampAngle` _returnvalue_roll -30.0 30.0) (`KismetMathLibrary.ClampAngle` _returnvalue_pitch -30.0 30.0) _returnvalue_yaw) false false))

(event `Grip Handler`
  (bind _carbody (`self.carBody`))
  (bind _returnvalue (`KismetMathLibrary.Normal` (`KismetMathLibrary.MakeVector` (.x (`SceneComponent.GetRightVector` _carbody)) (.y (`SceneComponent.GetRightVector` _carbody)))))
  (bind _returnvalue_2 (* _returnvalue (`KismetMathLibrary.Dot_VectorVector` (`SceneComponent.GetComponentVelocity` _carbody) _returnvalue)))
  (if (not (`self.Drifting`))
    (`PrimitiveComponent.AddForce` (`self.carBody`) (* (`KismetMathLibrary.NegateVector` _returnvalue_2) (`KismetMathLibrary.MapRangeClamped` (`KismetMathLibrary.VSize` _returnvalue_2) 350.0 1200.0 5000.0 7000.0)) "None" false)))

(event `EnhancedInput|/Game/Data/Input/IA_Accelerate`
  (params (ActionValue :type "Float (double-precision)") (ElapsedSeconds :type "Float (double-precision)") (TriggeredSeconds :type "Float (double-precision)") (InputAction :type "InputAction Object Reference" :default "/Game/Data/Input/IA_Accelerate.IA_Accelerate"))
  (:`Triggered`
    (`PrimitiveComponent.AddForceAtLocationLocal` (`self.carBody`) (`KismetMathLibrary.MakeVector` (* ActionValue (`self.Fwd Speed Max`)) 0.0 (* ActionValue -240000.0)) (0.0 0.0 0.0) "None")))

(event `FP_Thruster`
  (bind _frontright (`self.frontRight`))
  (bind _bpc_suspensionfp (`self.BPC_SuspensionFP`))
  (bind _returnvalue (`SceneComponent.K2_GetComponentLocation` _frontright))
  (bind _returnvalue_2 (`SceneComponent.K2_GetComponentLocation` (`self.frontRight`)))
  ;[1 1 1] Passenger Front
  (bind _outhit (`KismetSystemLibrary.LineTraceSingle` :`Start` _returnvalue :`End` (+ _returnvalue (* (`SceneComponent.GetUpVector` _frontright) -1.0 (`self.HoverMaxHeight_Front`))) :`TraceChannel` "TraceTypeQuery1" :`DrawDebugType` "ForOneFrame"))
  (bind (_bblockinghit _binitialoverlap _time _distance _location _impactpoint _normal _impactnormal) (`GameplayStatics.BreakHitResult` _outhit))
  (if _bblockinghit
    (set `self.onGround` true)
    (`/Game/Blueprints/Components/BPC_Suspension.Spring Compression` _bpc_suspensionfp (`self.Spring Constant`) (`self.Damping Coefficient`) (`self.HoverMaxHeight_Front`) (`self.carBody`) _returnvalue_2 _location _bblockinghit)
    (`PrimitiveComponent.AddForceAtLocation` (`self.carBody`) (* _impactnormal (`/Game/Blueprints/Components/BPC_Suspension.SuspensionForce` _bpc_suspensionfp)) (+ (* _impactnormal 1.0) _returnvalue_2) "None")
    (`SceneComponent.K2_SetWorldLocation` (`self.FRWheel`) (`KismetMathLibrary.MakeVector` (.x _impactpoint) (.y _impactpoint) (+ (.z _impactpoint) 20.0)) false false)
    (else
      (set `self.onGround` false))))

(event `FD_Thruster`
  (bind _frontleft (`self.frontLeft`))
  (bind _bpc_suspensionfd (`self.BPC_SuspensionFD`))
  (bind _returnvalue (`SceneComponent.K2_GetComponentLocation` _frontleft))
  ;[1 1 1] Driver Front
  (bind _outhit (`KismetSystemLibrary.LineTraceSingle` :`Start` _returnvalue :`End` (+ _returnvalue (* (`SceneComponent.GetUpVector` _frontleft) -1.0 (`self.HoverMaxHeight_Front`))) :`TraceChannel` "TraceTypeQuery1" :`DrawDebugType` "ForOneFrame"))
  (bind (_bblockinghit _binitialoverlap _time _distance _location _impactpoint _normal _impactnormal) (`GameplayStatics.BreakHitResult` _outhit))
  (if _bblockinghit
    (set `self.onGround` true)
    (`/Game/Blueprints/Components/BPC_Suspension.Spring Compression` _bpc_suspensionfd (`self.Spring Constant`) (`self.Damping Coefficient`) (`self.HoverMaxHeight_Front`) (`self.carBody`) (`SceneComponent.K2_GetComponentLocation` (`self.frontLeft`)) _impactpoint _bblockinghit)
    (`PrimitiveComponent.AddForceAtLocation` (`self.carBody`) (* _impactnormal (`/Game/Blueprints/Components/BPC_Suspension.SuspensionForce` _bpc_suspensionfd)) (+ (* _impactnormal 1.0) (`SceneComponent.K2_GetComponentLocation` (`self.frontLeft`))) "None")
    (`SceneComponent.K2_SetWorldLocation` (`self.FLWheel`) (`KismetMathLibrary.MakeVector` (.x _impactpoint) (.y _impactpoint) (+ (.z _impactpoint) 20.0)) false false)
    (else
      (set `self.onGround` false))))

(event `EnhancedInput|/Game/Data/Input/IA_Turn`
  (params (ActionValue :type "Float (double-precision)") (ElapsedSeconds :type "Float (double-precision)") (TriggeredSeconds :type "Float (double-precision)") (InputAction :type "InputAction Object Reference" :default "/Game/Data/Input/IA_Turn.IA_Turn"))
  (bind _returnvalue (`KismetMathLibrary.MapRangeClamped` ActionValue -1.0 1.0 -25.0 25.0))
  (bind _frwheel (`self.FRWheel`))
  (bind _flwheel (`self.FLWheel`))
  (bind _carbody (`self.carBody`))
  (bind _carbody_2 (`self.carBody`))
  (bind _frwheel_2 (`self.FRWheel`))
  (bind _flwheel_2 (`self.FLWheel`))
  (bind _returnvalue_2 (`KismetMathLibrary.MakeVector` 0.0 (* ActionValue 60000.0)))
  (bind _returnvalue_3 (`KismetMathLibrary.MakeVector` 0.0 (* ActionValue 5000.0)))
  (bind (_relativerotation_roll _relativerotation_pitch) (`KismetMathLibrary.BreakRotator` (`SceneComponent.RelativeRotation` _flwheel_2)))
  (bind (_relativerotation_roll_2 _relativerotation_pitch_2) (`KismetMathLibrary.BreakRotator` (`SceneComponent.RelativeRotation` _frwheel)))
  (bind (_relativerotation_roll_3 _relativerotation_pitch_3) (`KismetMathLibrary.BreakRotator` (`SceneComponent.RelativeRotation` _frwheel_2)))
  (bind (_relativerotation_roll_4 _relativerotation_pitch_4) (`KismetMathLibrary.BreakRotator` (`SceneComponent.RelativeRotation` _flwheel)))
  (:`Triggered`
    (`PrimitiveComponent.SetCenterOfMass` (`self.carBody`) (-35.0 0.0 0.0) "None")
    (switch `int` (`KismetMathLibrary.Round` (`KismetMathLibrary.SignOfFloat` ActionValue))
      (:`-1`
        (`PrimitiveComponent.AddForceAtLocationLocal` _carbody _returnvalue_2 (`SceneComponent.RelativeLocation` (`self.frontLeft`)) "None")
        (`PrimitiveComponent.AddForceAtLocationLocal` _carbody_2 _returnvalue_3 (`SceneComponent.RelativeLocation` (`self.rearRight`)) "None"))
      (:`1`
        (`PrimitiveComponent.AddForceAtLocationLocal` _carbody _returnvalue_2 (`SceneComponent.RelativeLocation` (`self.frontRight`)) "None")
        (`PrimitiveComponent.AddForceAtLocationLocal` _carbody_2 _returnvalue_3 (`SceneComponent.RelativeLocation` (`self.rearLeft`)) "None")))
    (`SceneComponent.K2_SetRelativeRotation` _flwheel_2 (`KismetMathLibrary.MakeRotator` _relativerotation_roll _relativerotation_pitch _returnvalue) false false)
    (`SceneComponent.K2_SetRelativeRotation` _frwheel_2 (`KismetMathLibrary.MakeRotator` _relativerotation_roll_3 _relativerotation_pitch_3 _returnvalue) false false))
  (:`Canceled`
    (`SceneComponent.K2_SetRelativeRotation` _frwheel (`KismetMathLibrary.MakeRotator` _relativerotation_roll_2 _relativerotation_pitch_2) false false :!label _label_2)
    (`SceneComponent.K2_SetRelativeRotation` _flwheel (`KismetMathLibrary.MakeRotator` _relativerotation_roll_4 _relativerotation_pitch_4) false false))
  (:`Completed`
    (goto _label_2)))

(event `RD_Thruster`
  (bind _rearleft (`self.rearLeft`))
  (bind _bpc_suspensionrd (`self.BPC_SuspensionRD`))
  (bind _returnvalue (`SceneComponent.K2_GetComponentLocation` _rearleft))
  (bind _returnvalue_2 (`SceneComponent.K2_GetComponentLocation` (`self.rearLeft`)))
  ;[1 1 1] Driver Rear
  (bind _outhit (`KismetSystemLibrary.LineTraceSingle` :`Start` _returnvalue :`End` (+ _returnvalue (* (`SceneComponent.GetUpVector` _rearleft) -1.0 (`self.HoverMaxHeight_Rear`))) :`TraceChannel` "TraceTypeQuery1" :`DrawDebugType` "ForOneFrame"))
  (bind (_bblockinghit _binitialoverlap _time _distance _location _impactpoint _normal _impactnormal) (`GameplayStatics.BreakHitResult` _outhit))
  (if _bblockinghit
    (set `self.onGround` true)
    (`/Game/Blueprints/Components/BPC_Suspension.Spring Compression` _bpc_suspensionrd (`self.Spring Constant`) (`self.Damping Coefficient`) (`self.HoverMaxHeight_Front`) (`self.carBody`) _returnvalue_2 _location _bblockinghit)
    (`PrimitiveComponent.AddForceAtLocation` (`self.carBody`) (* _impactnormal (`/Game/Blueprints/Components/BPC_Suspension.SuspensionForce` _bpc_suspensionrd)) (+ (* _impactnormal 1.0) _returnvalue_2) "None")
    (`SceneComponent.K2_SetWorldLocation` (`self.RLWheel`) (`KismetMathLibrary.MakeVector` (.x _impactpoint) (.y _impactpoint) (+ (.z _impactpoint) 20.0)) false false)
    (else
      (set `self.onGround` false))))

(event `RP_Thruster`
  (bind _rearright (`self.rearRight`))
  (bind _bpc_suspensionrp (`self.BPC_SuspensionRP`))
  (bind _returnvalue (`SceneComponent.K2_GetComponentLocation` _rearright))
  (bind _returnvalue_2 (`SceneComponent.K2_GetComponentLocation` (`self.rearRight`)))
  ;[1 1 1] Passenger Rear
  (bind _outhit (`KismetSystemLibrary.LineTraceSingle` :`Start` _returnvalue :`End` (+ _returnvalue (* (`SceneComponent.GetUpVector` _rearright) -1.0 (`self.HoverMaxHeight_Rear`))) :`TraceChannel` "TraceTypeQuery1" :`DrawDebugType` "ForDuration"))
  (bind (_bblockinghit _binitialoverlap _time _distance _location _impactpoint _normal _impactnormal) (`GameplayStatics.BreakHitResult` _outhit))
  (if _bblockinghit
    (set `self.onGround` true)
    (`/Game/Blueprints/Components/BPC_Suspension.Spring Compression` _bpc_suspensionrp (`self.Spring Constant`) (`self.Damping Coefficient`) (`self.HoverMaxHeight_Front`) (`self.carBody`) _returnvalue_2 _location _bblockinghit)
    (`PrimitiveComponent.AddForceAtLocation` (`self.carBody`) (* _impactnormal (`/Game/Blueprints/Components/BPC_Suspension.SuspensionForce` _bpc_suspensionrp)) (+ (* _impactnormal 1.0) _returnvalue_2) "None")
    (`SceneComponent.K2_SetWorldLocation` (`self.RRWheel`) (`KismetMathLibrary.MakeVector` (.x _impactpoint) (.y _impactpoint) (+ (.z _impactpoint) 20.0)) false false)
    (else
      (set `self.onGround` false))))

(event `ItemUse`)

(event `EnhancedInput|/Game/Data/Input/IA_ItemUse`
  (params (ActionValue :type Boolean) (ElapsedSeconds :type "Float (double-precision)") (TriggeredSeconds :type "Float (double-precision)") (InputAction :type "InputAction Object Reference" :default "/Game/Data/Input/IA_ItemUse.IA_ItemUse"))
  (:`Triggered`
    (if (!= (`self.CurrentItem`) 0)
      (`self.ItemUse`)
      (set `self.CurrentItem` 0))))

(event `Hit`
  (params (HitByID :type Integer))
  (switch `int` HitByID))

(event `ItemGive`
  (switch `int` (`KismetMathLibrary.RandomIntegerInRange` 1 4)
    (:`1`
      (set `self.CurrentItem` 1)
      (`KismetSystemLibrary.PrintString` "Gave Item1"))
    (:`2`
      (set `self.CurrentItem` 2)
      (`KismetSystemLibrary.PrintString` "Gave Item2"))
    (:`3`
      (set `self.CurrentItem` 3)
      (`KismetSystemLibrary.PrintString` "Gave Item3"))
    (:`4`
      (set `self.CurrentItem` 4)
      (`KismetSystemLibrary.PrintString` "Gave Item4"))))

(event `CustomEvent`)

(fn `Spring Compression`
  (params (`Current Height` :type "Float (double-precision)"))
  (returns (`Total Force` :type "Float (double-precision)"))
  (bind _returnvalue (+ (* (`self.Spring Constant`) (`self.Compression`)) (* (* (`self.Damping Coefficient`) -1.0) (`self.WheelVelocity`))))
  (set `self.Compression` (- (- (`self.HoverMaxHeight_Front`) 10.0) `Current Height`))
  (set `self.WheelAcceleration` (/ _returnvalue (`PrimitiveComponent.GetMass` (`self.carBody`))))
  (set `self.WheelVelocity` (+ (`self.WheelVelocity`) (* (`self.WheelAcceleration`) (`GameplayStatics.GetWorldDeltaSeconds`))))
  (return _returnvalue))

(fn `UserConstructionScript`)