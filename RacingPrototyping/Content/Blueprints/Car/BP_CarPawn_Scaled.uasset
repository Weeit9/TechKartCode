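; Kart-racer car pawn with physics driving, items and a per-player placement HUD, tuned by a player data asset.
; Tick runs four line-trace thrusters for curve-based suspension, lateral grip through a traction timeline, and roll/pitch clamping.
; Input applies forces for throttle and steering, toggles drifting and uses items (shells, banana, speed-up).
; Race progress and laps derive from BP_RaceSpline distance; drift-boost charging is disconnected, and random item grants exclude Bullet Bill.
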(event `EnhancedInput|/Game/Data/Input/IA_Drift`
  (params (ActionValue :type Boolean) (ElapsedSeconds :type "Float (double-precision)") (TriggeredSeconds :type "Float (double-precision)") (InputAction :type "InputAction Object Reference" :default "/Game/Data/Input/IA_Drift.IA_Drift"))
  ;[0.05769 0.06378 0.15 0.5] Drifting
  (:`Triggered`
    (set `self.Drifting` true))
  (:`Canceled`
    (set `self.Drifting` false :!label _label))
  (:`Completed`
    (goto _label)))

(event `On Ground Check`
  ;[0 0.15 0.1189 0.5] Feel Controls
  ;;[0 0 0 0.5] Ground Check
  (if (not (`self.onGround`))
    (`PrimitiveComponent.AddForce` (`self.carBody`) (0.0 0.0 -500000.0) "None" false)))

(event `Clamp Rotation`
  (bind _carbody (`self.carBody`))
  (bind (_returnvalue_roll _returnvalue_pitch _returnvalue_yaw) (`KismetMathLibrary.BreakRotator` (`SceneComponent.K2_GetComponentRotation` _carbody)))
  ;[0 0.15 0.1189 0.5] Feel Controls
  ;;[0.01042 0.01042 0.01042 0.5] Clamp Rotation
  (`SceneComponent.K2_SetWorldRotation` _carbody (`KismetMathLibrary.MakeRotator` (`KismetMathLibrary.ClampAngle` _returnvalue_roll -30.0 30.0) (`KismetMathLibrary.ClampAngle` _returnvalue_pitch -30.0 30.0) _returnvalue_yaw) false false))

(event `Grip Handler`
  (bind _griprange (`self.GripRange`))
  (bind _carbody (`self.carBody`))
  (bind _returnvalue (`KismetMathLibrary.Normal` (`KismetMathLibrary.MakeVector` (.x (`SceneComponent.GetRightVector` _carbody)) (.y (`SceneComponent.GetRightVector` _carbody)))))
  (bind _returnvalue_2 (* _returnvalue (`KismetMathLibrary.Dot_VectorVector` (`SceneComponent.GetComponentVelocity` _carbody) _returnvalue)))
  ;[0 0.15 0.1189 0.5] Feel Controls
  ;;[0 0 0 0.5] Grip Handling
  (if (`self.Drifting`)
    (bind (_direction _lerp_alpha) (`Timeline|RegainTraction` :!via `SetNewTime` :!label _label_2)
      (:`Update`
        (bind _returnvalue_3 (`KismetMathLibrary.Lerp` 0.0 (`KismetMathLibrary.VSize` _returnvalue_2) _lerp_alpha))
        (`PrimitiveComponent.AddForce` (`self.carBody`) (* (`KismetMathLibrary.NegateVector` _returnvalue_2) (`KismetMathLibrary.SelectFloat` 0.0 (`KismetMathLibrary.MapRangeClamped` _returnvalue_3 200.0 1200.0 (`|GetArrayItem` _griprange) (`|GetArrayItem` _griprange 1)) (< _returnvalue_3 200.0))) "None" false)))
    (else
      (goto _label_2))))

(event `Update Placement HUD`
  (set `/Game/UI/RacePlacement_WID.Placement#` (`self.Current Place`) (`/Game/UI/RaceHUD_WID.RacePlacement_WID` (`self.HudRef`))))

(event `self.Update Race Placement`
  (params (`New Place` :type Integer))
  (set `self.Current Place` `New Place`))

(event `Boost`
  ;[0.04636 0.04573 0.15 0.5] Turning
  ;; Boost
  (switch `int` (`self.Boost Level`)
    (:`1`
      (set `self.Current Max Speed` (* (`self.Fwd Speed Max`) 1.25))
      (`PrimitiveComponent.AddForceAtLocationLocal` (`self.carBody`) (40000000.0 0.0 0.0) (0.0 0.0 0.0) "None")
      (`KismetSystemLibrary.Delay` 1.0)
      (set `self.Current Max Speed` (`self.Fwd Speed Max`)))
    (:`2`
      (set `self.Current Max Speed` (* (`self.Fwd Speed Max`) 1.35))
      (`PrimitiveComponent.AddForceAtLocationLocal` (`self.carBody`) (47500000.0 0.0 0.0) (0.0 0.0 0.0) "None")
      (`KismetSystemLibrary.Delay` 1.5)
      (set `self.Current Max Speed` (`self.Fwd Speed Max`)))
    (:`3`
      (set `self.Current Max Speed` (* (`self.Fwd Speed Max`) 1.75))
      (`PrimitiveComponent.AddForceAtLocationLocal` (`self.carBody`) (60000000.0 0.0 0.0) (0.0 0.0 0.0) "None")
      (`KismetSystemLibrary.Delay` 2.0)
      (set `self.Current Max Speed` (`self.Fwd Speed Max`)))))

(event `self.ReceiveTick`
  (params (DeltaSeconds :type "Float (single-precision)"))
  ; Tick
  (`self.FD_Thruster`)
  (`self.FP_Thruster`)
  (`self.RD_Thruster`)
  (`self.RP_Thruster`)
  (`self.Grip Handler`)
  (`self.Clamp Rotation`)
  (`self.Update Placement HUD`))

(event `EnhancedInput|/Game/Data/Input/IA_Accelerate`
  (params (ActionValue :type "Float (double-precision)") (ElapsedSeconds :type "Float (double-precision)") (TriggeredSeconds :type "Float (double-precision)") (InputAction :type "InputAction Object Reference" :default "/Game/Data/Input/IA_Accelerate.IA_Accelerate"))
  ;[0.02625 0.04131 0.15 0.5] Acceleration
  (:`Triggered`
    (`PrimitiveComponent.AddForceAtLocationLocal` (`self.carBody`) (`KismetMathLibrary.MakeVector` (* ActionValue (`self.Fwd Speed Max`)) 0.0 (* ActionValue -240000.0)) (0.0 0.0 0.0) "None")))

(event `EnhancedInput|/Game/Data/Input/IA_Turn`
  (params (ActionValue :type "Float (double-precision)") (ElapsedSeconds :type "Float (double-precision)") (TriggeredSeconds :type "Float (double-precision)") (InputAction :type "InputAction Object Reference" :default "/Game/Data/Input/IA_Turn.IA_Turn"))
  (bind _returnvalue (`KismetMathLibrary.MapRangeClamped` ActionValue -1.0 1.0 -25.0 25.0))
  (bind _frwheel (`self.FRWheel`))
  (bind _flwheel (`self.FLWheel`))
  (bind _frwheel_2 (`self.FRWheel`))
  (bind _flwheel_2 (`self.FLWheel`))
  (bind _carbody (`self.carBody`))
  (bind _carbody_2 (`self.carBody`))
  (bind _returnvalue_2 (`KismetMathLibrary.MakeVector` 0.0 (* ActionValue 200000.0)))
  (bind (_relativerotation_roll _relativerotation_pitch) (`KismetMathLibrary.BreakRotator` (`SceneComponent.RelativeRotation` _frwheel_2)))
  (bind (_relativerotation_roll_2 _relativerotation_pitch_2) (`KismetMathLibrary.BreakRotator` (`SceneComponent.RelativeRotation` _flwheel)))
  (bind (_relativerotation_roll_3 _relativerotation_pitch_3) (`KismetMathLibrary.BreakRotator` (`SceneComponent.RelativeRotation` _flwheel_2)))
  (bind (_relativerotation_roll_4 _relativerotation_pitch_4) (`KismetMathLibrary.BreakRotator` (`SceneComponent.RelativeRotation` _frwheel)))
  (bind _returnvalue_3 (`KismetMathLibrary.MakeVector` 0.0 (* (* ActionValue 50000.0) (`GameplayStatics.GetWorldDeltaSeconds`))))
  ;[0.04636 0.04573 0.15 0.5] Turning
  (:`Triggered`
    (if (`self.onGround`)
      (`PrimitiveComponent.SetCenterOfMass` (`self.carBody`) (-35.0 0.0 0.0) "None")
      (switch `int` (`KismetMathLibrary.Round` (`KismetMathLibrary.SignOfFloat` ActionValue))
        (:`-1`
          (`PrimitiveComponent.AddForceAtLocationLocal` _carbody_2 _returnvalue_2 (`SceneComponent.RelativeLocation` (`self.frontLeft`)) "None")
          (`PrimitiveComponent.AddForceAtLocationLocal` _carbody _returnvalue_3 (`SceneComponent.RelativeLocation` (`self.rearRight`)) "None"))
        (:`1`
          (`PrimitiveComponent.AddForceAtLocationLocal` _carbody_2 _returnvalue_2 (`SceneComponent.RelativeLocation` (`self.frontRight`)) "None")
          (`PrimitiveComponent.AddForceAtLocationLocal` _carbody _returnvalue_3 (`SceneComponent.RelativeLocation` (`self.rearLeft`)) "None")))
      (`SceneComponent.K2_SetRelativeRotation` _flwheel_2 (`KismetMathLibrary.MakeRotator` _relativerotation_roll_3 _relativerotation_pitch_3 _returnvalue) false false)
      (`SceneComponent.K2_SetRelativeRotation` _frwheel_2 (`KismetMathLibrary.MakeRotator` _relativerotation_roll _relativerotation_pitch _returnvalue) false false)))
  (:`Canceled`
    (`SceneComponent.K2_SetRelativeRotation` _frwheel (`KismetMathLibrary.MakeRotator` _relativerotation_roll_4 _relativerotation_pitch_4) false false :!label _label_3)
    (`SceneComponent.K2_SetRelativeRotation` _flwheel (`KismetMathLibrary.MakeRotator` _relativerotation_roll_2 _relativerotation_pitch_2) false false))
  (:`Completed`
    (goto _label_3)))

(event `FP_Thruster`
  (bind _frontright (`self.frontRight`))
  (bind _returnvalue (`SceneComponent.K2_GetComponentLocation` _frontright))
  ;[0.15 0 0.02154 0.5] Suspension
  ;;[1 1 1] Passenger Front
  (bind _outhit (`KismetSystemLibrary.LineTraceSingle` :`Start` _returnvalue :`End` (+ _returnvalue (* (`SceneComponent.GetUpVector` _frontright) -1.0 (`self.HoverMaxHeight_Front`))) :`TraceChannel` "TraceTypeQuery1" :`DrawDebugType` "ForOneFrame"))
  (bind (_bblockinghit _binitialoverlap _time _distance _location _impactpoint _normal _impactnormal) (`GameplayStatics.BreakHitResult` _outhit))
  (if _bblockinghit
    (set `self.onGround` true)
    (`PrimitiveComponent.AddForceAtLocation` (`self.carBody`) (/ (* (`KismetMathLibrary.GetRuntimeFloatCurveValue` (`self.Curve`) (/ _distance (`self.HoverMaxHeight_Front`))) _impactnormal) (`GameplayStatics.GetWorldDeltaSeconds`)) (+ (* _impactnormal 1.0) (`SceneComponent.K2_GetComponentLocation` (`self.frontRight`))) "None")
    (`SceneComponent.K2_SetWorldLocation` (`self.FRWheel`) (`KismetMathLibrary.MakeVector` (.x _impactpoint) (.y _impactpoint) (+ (.z _impactpoint) 13.0)) false false)
    (else
      (set `self.onGround` false))))

(event `FD_Thruster`
  (bind _frontleft (`self.frontLeft`))
  (bind _returnvalue (`SceneComponent.K2_GetComponentLocation` _frontleft))
  ;[0.15 0 0.02154 0.5] Suspension
  ;;[1 1 1] Driver Front
  (bind _outhit (`KismetSystemLibrary.LineTraceSingle` :`Start` _returnvalue :`End` (+ _returnvalue (* (`SceneComponent.GetUpVector` _frontleft) -1.0 (`self.HoverMaxHeight_Front`))) :`TraceChannel` "TraceTypeQuery1" :`DrawDebugType` "ForOneFrame"))
  (bind (_bblockinghit _binitialoverlap _time _distance _location _impactpoint _normal _impactnormal) (`GameplayStatics.BreakHitResult` _outhit))
  (if _bblockinghit
    (set `self.onGround` true)
    (`PrimitiveComponent.AddForceAtLocation` (`self.carBody`) (/ (* (`KismetMathLibrary.GetRuntimeFloatCurveValue` (`self.Curve`) (/ _distance (`self.HoverMaxHeight_Front`))) _impactnormal) (`GameplayStatics.GetWorldDeltaSeconds`)) (+ (* _impactnormal 1.0) (`SceneComponent.K2_GetComponentLocation` (`self.frontLeft`))) "None")
    (`SceneComponent.K2_SetWorldLocation` (`self.FLWheel`) (`KismetMathLibrary.MakeVector` (.x _impactpoint) (.y _impactpoint) (+ (.z _impactpoint) 13.0)) false false)
    (else
      (set `self.onGround` false))))

(event `self.ReceiveBeginPlay`
  ;[0.03866 0.15 0.0326 0.5] Begin Play
  (bind _returnvalue (`GameplayStatics.GetActorOfClass` "/Game/Blueprints/Spline/BP_RaceSpline.BP_RaceSpline_C"))
  (bind _output_get (set `self.Track` _returnvalue))
  (set `self.SplineLength` (`SplineComponent.GetSplineLength` (`/Game/Blueprints/Spline/BP_RaceSpline.SplineToFollow` _output_get)))
  (`KismetSystemLibrary.K2_SetTimerDelegate` (`|CreateDelegate` :!event `RaceProgressTracker`) 0.3 true)
  (bind _returnvalue_2 (`|CreateWidget` "/Game/UI/RaceHUD_WID.RaceHUD_WID_C" (`GameplayStatics.GetPlayerController` (`self.Player Index`))))
  (bind _output_get_2 (set `self.HudRef` _returnvalue_2))
  (`UserWidget.AddToPlayerScreen` _output_get_2 0))

(event `RD_Thruster`
  (bind _rearleft (`self.rearLeft`))
  (bind _returnvalue (`SceneComponent.K2_GetComponentLocation` _rearleft))
  ;[0.15 0 0.02154 0.5] Suspension
  ;;[1 1 1] Driver Rear
  (bind _outhit (`KismetSystemLibrary.LineTraceSingle` :`Start` _returnvalue :`End` (+ _returnvalue (* (`SceneComponent.GetUpVector` _rearleft) -1.0 (`self.HoverMaxHeight_Rear`))) :`TraceChannel` "TraceTypeQuery1" :`DrawDebugType` "ForOneFrame"))
  (bind (_bblockinghit _binitialoverlap _time _distance _location _impactpoint _normal _impactnormal) (`GameplayStatics.BreakHitResult` _outhit))
  (if _bblockinghit
    (set `self.onGround` true)
    (`PrimitiveComponent.AddForceAtLocation` (`self.carBody`) (/ (* (`KismetMathLibrary.GetRuntimeFloatCurveValue` (`self.Curve`) (/ _distance (`self.HoverMaxHeight_Front`))) _impactnormal) (`GameplayStatics.GetWorldDeltaSeconds`)) (+ (* _impactnormal 1.0) (`SceneComponent.K2_GetComponentLocation` (`self.rearLeft`))) "None")
    (`SceneComponent.K2_SetWorldLocation` (`self.RLWheel`) (`KismetMathLibrary.MakeVector` (.x _impactpoint) (.y _impactpoint) (+ (.z _impactpoint) 13.0)) false false)
    (else
      (set `self.onGround` false))))

(event `RP_Thruster`
  (bind _rearright (`self.rearRight`))
  (bind _returnvalue (`SceneComponent.K2_GetComponentLocation` _rearright))
  ;[0.15 0 0.02154 0.5] Suspension
  ;;[1 1 1] Passenger Rear
  (bind _outhit (`KismetSystemLibrary.LineTraceSingle` :`Start` _returnvalue :`End` (+ _returnvalue (* (`SceneComponent.GetUpVector` _rearright) -1.0 (`self.HoverMaxHeight_Rear`))) :`TraceChannel` "TraceTypeQuery1" :`DrawDebugType` "ForDuration"))
  (bind (_bblockinghit _binitialoverlap _time _distance _location _impactpoint _normal _impactnormal) (`GameplayStatics.BreakHitResult` _outhit))
  (if _bblockinghit
    (set `self.onGround` true)
    (`PrimitiveComponent.AddForceAtLocation` (`self.carBody`) (/ (* _impactnormal (`KismetMathLibrary.GetRuntimeFloatCurveValue` (`self.Curve`) (/ _distance (`self.HoverMaxHeight_Front`)))) (`GameplayStatics.GetWorldDeltaSeconds`)) (+ (* _impactnormal 1.0) (`SceneComponent.K2_GetComponentLocation` (`self.rearRight`))) "None")
    (`SceneComponent.K2_SetWorldLocation` (`self.RRWheel`) (`KismetMathLibrary.MakeVector` (.x _impactpoint) (.y _impactpoint) (+ (.z _impactpoint) 13.0)) false false)
    (else
      (set `self.onGround` false))))

(event `EnhancedInput|/Game/Data/Input/IA_ItemUse`
  (params (ActionValue :type Boolean) (ElapsedSeconds :type "Float (double-precision)") (TriggeredSeconds :type "Float (double-precision)") (InputAction :type "InputAction Object Reference" :default "/Game/Data/Input/IA_ItemUse.IA_ItemUse"))
  ;[0.15 0.06341 0.001801 0.5] Item Handling
  ;;[0.05769 0.06378 0.15 0.5] Item Use
  (:`Triggered`
    (if (!= (`self.CurrentItem`) 0)
      (`self.ItemUse`)
      (set `self.CurrentItem` 0))))

(event `RaceProgressTracker`
  (bind _splinetofollow (`/Game/Blueprints/Spline/BP_RaceSpline.SplineToFollow` (`self.Track`)))
  (bind _returnvalue (`SplineComponent.GetDistanceAlongSplineAtLocation` _splinetofollow (`SplineComponent.FindLocationClosestToWorldLocation` _splinetofollow (`SceneComponent.K2_GetComponentLocation` (`self.carBody`)) "World") "World"))
  (bind _returnvalue_2 (/ _returnvalue (`self.SplineLength`)))
  (if (`KismetMathLibrary.InRange_FloatFloat` _returnvalue_2 0.45 0.6)
    (set `self.JustDidLap` false))
  (if (< _returnvalue_2 0.999)
    (set `self.DistanceAlongTrack` _returnvalue)
    (elif (not (`self.JustDidLap`))
      (`/Engine/EditorBlueprintResources/StandardMacros.IncrementInt` (`self.Lap#`)
        (:`  `
          (set `self.JustDidLap` true)
          (`KismetSystemLibrary.PrintString` "Lap")))))
  (`self.%OfRaceDone`))

(event `BulletBill`
  (bind _splinetofollow (`/Game/Blueprints/Spline/BP_RaceSpline.SplineToFollow` (`self.Track`)))
  ;[0.15 0.06341 0.001801 0.5] Item Handling
  ;; Bullet Bill
  (bind _output_get (set `self.CurrentSplineDistance` (+ (`self.CurrentSplineDistance`) (* (`self.BulletBillSpeed`) (`GameplayStatics.GetWorldDeltaSeconds`)))))
  (bind (_returnvalue_x _returnvalue_y _returnvalue_z) (`KismetMathLibrary.BreakVector` (`SplineComponent.GetLocationAtDistanceAlongSpline` _splinetofollow _output_get "World")))
  (`SceneComponent.K2_SetWorldLocationAndRotation` (`self.carBody`) (`KismetMathLibrary.MakeVector` _returnvalue_x _returnvalue_y (+ _returnvalue_z 150.0)) (`SplineComponent.GetRotationAtDistanceAlongSpline` _splinetofollow _output_get "World") false false))

(event `Hit`
  (params (HitByID :type Integer))
  ;[0.15 0.06341 0.001801 0.5] Item Handling
  ;; Hit
  (if (not (`self.InBulletBill`))
    (`self.DisableInput` null)
    (`KismetSystemLibrary.Delay` 2.0)
    (`self.EnableInput` null)))

(event `%OfRaceDone`
  (set `self.%RaceCompleted` (/ (`self.DistanceAlongTrack`) (`self.SplineLength`))))

(event `BulletBillTimer`
  ;[0.15 0.06341 0.001801 0.5] Item Handling
  ;; Bullet Bill
  (if (< (`self.BulletBillTime`) 5) :!label _label_4
    (`KismetSystemLibrary.Delay` 1.0)
    (set `self.BulletBillTime` (+ (`self.BulletBillTime`) 1))
    (goto _label_4)
    (else
      (set `self.InBulletBill` false))))

(event `ItemGive`
  ;[0.15 0.06341 0.001801 0.5] Item Handling
  ;; Item Give
  (switch `int` (`KismetMathLibrary.RandomIntegerInRange` 1 4)
    (:`1`
      (set `self.CurrentItem` 1)
      (`KismetSystemLibrary.PrintString` "Gave Item1"))
    (:`2`
      (set `self.CurrentItem` 2)
      (`KismetSystemLibrary.PrintString` "Gave Item2"))
    (:`3`
      (set `self.CurrentItem` 3)
      (`KismetSystemLibrary.PrintString` "Gave Item3"))
    (:`4`
      (set `self.CurrentItem` 4)
      (`KismetSystemLibrary.PrintString` "Gave Item4"))))

(event `ItemUse`
  (bind _returnvalue (`SceneComponent.K2_GetComponentRotation` (`self.carBody`)))
  (bind _returnvalue_2 (`SceneComponent.K2_GetComponentLocation` (`self.ItemSpawnerFront`)))
  ;[0.15 0.06341 0.001801 0.5] Item Handling
  ;; Item use
  (switch `int` (`self.CurrentItem`)
    (:`1`
      (`|SpawnActorFromClass` "/Game/Blueprints/Items/GreenShell_BP.GreenShell_BP_C" (`KismetMathLibrary.MakeTransform` _returnvalue_2 _returnvalue) "Undefined" "MultiplyWithRoot" null null))
    (:`2`
      (`|SpawnActorFromClass` "/Game/Blueprints/Items/RedShell_BP.RedShell_BP_C" (`KismetMathLibrary.MakeTransform` _returnvalue_2 _returnvalue) "Undefined" "MultiplyWithRoot" null null))
    (:`3`
      (`|SpawnActorFromClass` "/Game/Blueprints/Items/Banana_BP.Banana_BP_C" (`KismetMathLibrary.MakeTransform` (`SceneComponent.K2_GetComponentLocation` (`self.ItemSpawnerBack`)) _returnvalue) "Undefined" "MultiplyWithRoot" null null))
    (:`4`
      (set `self.Fwd Speed Max` (* (`self.Fwd Speed Max`) 1.5))
      (`KismetSystemLibrary.Delay` 3.0)
      (set `self.Fwd Speed Max` 4000000.0))
    (:`5`
      (set `self.CurrentSplineDistance` (`SplineComponent.FindInputKeyClosestToWorldLocation` (`/Game/Blueprints/Spline/BP_RaceSpline.SplineToFollow` (`self.Track`)) (`SceneComponent.K2_GetComponentLocation` (`self.carBody`))))
      (set `self.InBulletBill` true))))

(fn `Get Race Progress`
  (returns (`Distance Along Track` :type "Float (double-precision)"))
  (return (+ (`self.%RaceCompleted`) (`self.Lap#`))))

(fn `UserConstructionScript`
  (`StaticMeshComponent.SetStaticMesh` (`self.carMesh`) (`/Game/Blueprints/Car/PDA_CarSelection.CarMesh` (`self.PlayerDataAsset`)))
  (set `self.Fwd Speed Max` (`/Game/Blueprints/Car/PDA_CarSelection.Acceleration Speed` (`self.PlayerDataAsset`)))
  (set `self.GripRange` (`/Game/Blueprints/Car/PDA_CarSelection.Grip Factor` (`self.PlayerDataAsset`))))