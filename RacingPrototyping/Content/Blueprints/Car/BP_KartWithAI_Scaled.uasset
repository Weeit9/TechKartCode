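; Physics-driven racing kart pawn that takes player input or steering and throttle calls for AI, with AIC_VehicleAI as its AI controller class.
; Each tick, four wheel traces apply spring suspension and drive forces to the collision box, while ground-checked input sets acceleration and torque-based steering.
; The track spline feeds AI throttle and steering helpers and lap-plus-distance race progress, with a mid-track check preventing double-counted laps.
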(event `AIThrottle`
  (bind _returnvalue (`KismetMathLibrary.Dot_VectorVector` (`SplineComponent.FindDirectionClosestToWorldLocation` (`/Game/Blueprints/Spline/BP_RaceSpline.SplineToFollow` (`self.Track`)) (`self.K2_GetActorLocation`) "World") (`self.GetActorForwardVector`)))
  (set `self.AISetThrottle` (* (`KismetMathLibrary.FClamp` (`KismetMathLibrary.Abs` _returnvalue) 0.2 0.9) (`KismetMathLibrary.SignOfFloat` _returnvalue))))

(event `self.ReceiveBeginPlay`
  ; Event Begin Play
  (`KismetSystemLibrary.Delay` 0.2)
  (set `self.SplineLength` (`SplineComponent.GetSplineLength` (`/Game/Blueprints/Spline/BP_RaceSpline.SplineToFollow` (`self.Track`))))
  (set `self.AI_Controlled` true)
  (`KismetSystemLibrary.K2_SetTimerDelegate` (`|CreateDelegate` :!event `RaceProgressTracker`) 0.3 true))

(event `self.ReceiveTick`
  (params (DeltaSeconds :type "Float (single-precision)"))
  ; Event Tick
  (`|ExecutionSequence`
    (:`then_0`
      (`self.SuspensionCast` (`self.FrontRWheel`))
      (`self.SuspensionCast` (`self.BackRWheel`))
      (`self.SuspensionCast` (`self.BackLWheel`))
      (`self.SuspensionCast` (`self.FrontLWheel`))
      (`self.CalculateAcceleration`)
      (`self.TurnWheels`)
      (`self.GetTrackProgress`))
    (:`then_1`
      (if (`self.AI_Controlled`)
        _))))

(event `RaceProgressTracker`
  (bind _splinetofollow (`/Game/Blueprints/Spline/BP_RaceSpline.SplineToFollow` (`self.Track`)))
  (bind _returnvalue (`SplineComponent.GetDistanceAlongSplineAtLocation` _splinetofollow (`SplineComponent.FindLocationClosestToWorldLocation` _splinetofollow (`SceneComponent.K2_GetComponentLocation` (`self.Car_ColBox`)) "World") "World"))
  (bind _returnvalue_2 (/ _returnvalue (`self.SplineLength`)))
  (if (`KismetMathLibrary.InRange_FloatFloat` _returnvalue_2 0.45 0.6)
    (set `self.JustDidLap` false))
  (if (< _returnvalue_2 0.999)
    (set `self.DistanceAlongTrack` _returnvalue)
    (elif (not (`self.JustDidLap`))
      (`/Engine/EditorBlueprintResources/StandardMacros.IncrementInt` (`self.Lap#`)
        (:`  `
          (set `self.JustDidLap` true)))))
  (`self.%OfRaceDone`))

(event `%OfRaceDone`
  (set `self.%RaceCompleted` (/ (`self.DistanceAlongTrack`) (`self.SplineLength`))))

(event `self.SetThrottle`
  (params (Throttle :type "Float (double-precision)"))
  (set `self.AccelerationInput` (`KismetMathLibrary.FInterpTo` (`self.AccelerationInput`) (`KismetMathLibrary.SelectFloat` Throttle 0.0 (`self.isOnGround`)) (`GameplayStatics.GetWorldDeltaSeconds`) 0.8)))

(event `EnhancedInput|/Game/Data/Input/IA_Accelerate`
  (params (ActionValue :type "Float (double-precision)") (ElapsedSeconds :type "Float (double-precision)") (TriggeredSeconds :type "Float (double-precision)") (InputAction :type "InputAction Object Reference" :default "/Game/Data/Input/IA_Accelerate.IA_Accelerate"))
  ; Accelerate
  (:`Triggered`
    (set `self.AccelerationInput` (`KismetMathLibrary.FInterpTo` (`self.AccelerationInput`) (`KismetMathLibrary.SelectFloat` ActionValue 0.0 (`self.isOnGround`)) (`GameplayStatics.GetWorldDeltaSeconds`) 0.8))))

(event `EnhancedInput|/Game/Data/Input/IA_Turn`
  (params (ActionValue :type "Float (double-precision)") (ElapsedSeconds :type "Float (double-precision)") (TriggeredSeconds :type "Float (double-precision)") (InputAction :type "InputAction Object Reference" :default "/Game/Data/Input/IA_Turn.IA_Turn"))
  ; Steering
  (:`Triggered`
    (if (`self.isOnGround`)
      (set `self.TurnInput` ActionValue)
      (`PrimitiveComponent.AddTorqueInRadians` (`self.Car_ColBox`) (`KismetMathLibrary.MakeVector` 0.0 0.0 (* (`self.TurnInput`) 10000000.0 (`self.AccelerationInput`))) "None" false)))
  (:`Completed`
    (set `self.TurnInput` 0.0)))

(event `TurnWheels`
  (bind (_relativerotation_roll _relativerotation_pitch _relativerotation_yaw) (`KismetMathLibrary.BreakRotator` (`SceneComponent.RelativeRotation` (`self.FrontLWheel`))))
  ; TurnWheels
  (`SceneComponent.K2_SetRelativeRotation` (`self.FrontRWheel`) (`KismetMathLibrary.MakeRotator` 0.0 0.0 (`KismetMathLibrary.FInterpTo` _relativerotation_yaw (* (`self.TurnInput`) (`self.TurnRadius`)) (`GameplayStatics.GetWorldDeltaSeconds`) 3.0)) false false)
  (`SceneComponent.K2_SetRelativeRotation` (`self.FrontLWheel`) (`KismetMathLibrary.MakeRotator` 0.0 0.0 (`KismetMathLibrary.FInterpTo` _relativerotation_yaw (* (`self.TurnInput`) (`self.TurnRadius`)) (`GameplayStatics.GetWorldDeltaSeconds`) 3.0)) false false))

(event `self.SetSteering`
  (params (Steering :type "Float (double-precision)") (SteeringAdjust :type "Float (double-precision)"))
  (if (`self.isOnGround`)
    (bind _output_get (set `self.TurnInput` Steering))
    (`PrimitiveComponent.AddTorqueInRadians` (`self.Car_ColBox`) (`KismetMathLibrary.MakeVector` 0.0 0.0 (* (+ _output_get SteeringAdjust) 10000000.0 (`self.AccelerationInput`))) "None" false)))

(fn `AI_AccelerateKart`
  (params (Throttle :type "Float (double-precision)"))
  (set `self.AccelerationInput` (`KismetMathLibrary.FInterpTo` (`self.AccelerationInput`) (`KismetMathLibrary.SelectFloat` Throttle 0.0 (`self.isOnGround`)) (`GameplayStatics.GetWorldDeltaSeconds`) 0.8)))

(fn `AI_SteerKart`
  (params (SteeringDir :type "Float (double-precision)"))
  (if (`self.isOnGround`)
    (`PrimitiveComponent.AddTorqueInRadians` (`self.Car_ColBox`) (`KismetMathLibrary.MakeVector` 0.0 0.0 (* SteeringDir 500000.0 (`self.AccelerationInput`))) "None" false)))

(fn `AISteeringNew`)

(fn `CalculateAcceleration`
  (bind _acceleration (`self.Acceleration`))
  (set `self.Acceleration` (* (`KismetMathLibrary.Lerp` 0.0 15000.0 (`self.AccelerationInput`)) (`self.AccelerationInput`)))
  (if (`self.isOnGround`)
    (set `self.AccelerationInput` (`KismetMathLibrary.FInterpTo` (`self.AccelerationInput`) 0.0 (`GameplayStatics.GetWorldDeltaSeconds`) 0.6))
    (`SceneComponent.K2_AddLocalRotation` (`self.WheelMesh_BL`) (`KismetMathLibrary.MakeRotator` 0.0 (* (/ _acceleration 1000.0) (`self.AccelerationInput`))) false false)
    (`SceneComponent.K2_AddLocalRotation` (`self.WheelMesh_FL`) (`KismetMathLibrary.MakeRotator` 0.0 (* (/ _acceleration 1000.0) (`self.AccelerationInput`))) false false)
    (`SceneComponent.K2_AddLocalRotation` (`self.WheelMesh_BR`) (`KismetMathLibrary.MakeRotator` 0.0 (* (/ _acceleration -1000.0) (`self.AccelerationInput`))) false false)
    (`SceneComponent.K2_AddLocalRotation` (`self.WheelMesh_FR`) (`KismetMathLibrary.MakeRotator` 0.0 (* (/ _acceleration -1000.0) (`self.AccelerationInput`))) false false)))

(fn `CalculateAISteering_New`
  (returns (SteeringInput :type "Float (double-precision)"))
  (bind _returnvalue (`self.K2_GetActorLocation`))
  (bind _locationtosteerto (message `/Game/Blueprints/Interface/BPI_isAIPath.GetClosestLocationToAIPath` (`self.Track`) _returnvalue 0.0 0))
  (bind (_returnvalue_roll _returnvalue_pitch _returnvalue_yaw) (`KismetMathLibrary.BreakRotator` (`KismetMathLibrary.NormalizedDeltaRotator` (`KismetMathLibrary.FindLookAtRotation` _returnvalue _locationtosteerto) (`self.K2_GetActorRotation`))))
  (return (`KismetMathLibrary.MapRangeClamped` _returnvalue_yaw -10.0 10.0 -1.0 1.0)))

(fn `Get Race Progress`
  (returns (`Distance Along Track` :type "Float (double-precision)"))
  (return (+ (`self.%RaceCompleted`) (`self.Lap#`))))

(fn `GetAISteering`
  (returns (ReturnValue :type "Float (double-precision)"))
  (bind _returnvalue (`KismetMathLibrary.Dot_VectorVector` (`SplineComponent.FindDirectionClosestToWorldLocation` (`/Game/Blueprints/Spline/BP_RaceSpline.SplineToFollow` (`self.Track`)) (+ (`self.K2_GetActorLocation`) (* (`self.GetActorForwardVector`) (`KismetMathLibrary.RandomFloatInRange` 1.0 500.0))) "World") (`self.GetActorRightVector`)))
  (return (* _returnvalue (`self.Acceleration`) (`KismetMathLibrary.MultiplyMultiply_FloatFloat` (`KismetMathLibrary.Abs` _returnvalue) 1.0))))

(fn `GetCollisionBoxes`
  (returns (FrontBox :type "BoxComponent Object Reference") (LeftSideBox :type "BoxComponent Object Reference") (RightSideBOx :type "BoxComponent Object Reference"))
  (return (`self.FrontBox`) (`self.LeftSideBox`) (`self.RightSideBox`)))

(fn `GetCurrentSpeed`
  (returns (CurrentSpeed :type "Float (double-precision)"))
  (return (`KismetMathLibrary.VSize` (`self.GetVelocity`))))

(fn `GetFrontOfCar`
  (returns (FrontLocation :type "Vector Structure"))
  (return (`SceneComponent.K2_GetComponentLocation` (`self.FrontOfCar`))))

(fn `GetTrackProgress`)

(fn `isOnGround`
  (returns (ReturnValue :type Boolean))
  (bind _returnvalue (`self.K2_GetActorLocation`))
  (bind (_outhit _returnvalue_2) (`KismetSystemLibrary.LineTraceSingle` :`Start` _returnvalue :`End` (- _returnvalue 64.0) :`TraceChannel` "TraceTypeQuery1" :`DrawDebugType` "ForOneFrame"))
  (return _returnvalue_2))

(fn `SuspensionCast`
  (params (WheelComp :type "SceneComponent Object Reference"))
  (bind _returnvalue (`SceneComponent.K2_GetComponentLocation` WheelComp))
  (bind _car_colbox (`self.Car_ColBox`))
  (bind _returnvalue_2 (`SceneComponent.GetChildComponent` (`local.WheelComp`) 0))
  (bind (_relativelocation_x _relativelocation_y _relativelocation_z) (`KismetMathLibrary.BreakVector` (`SceneComponent.RelativeLocation` _returnvalue_2)))
  (bind _outhit (`KismetSystemLibrary.LineTraceSingle` _returnvalue (+ _returnvalue (* (`SceneComponent.GetUpVector` WheelComp) -60.0)) "TraceTypeQuery1"))
  (bind (_bblockinghit _binitialoverlap _time _distance _location _impactpoint _normal _impactnormal _physmat _hitactor _hitcomponent _hitbonename _bonename _hititem _elementindex _faceindex _tracestart _traceend) (`GameplayStatics.BreakHitResult` _outhit))
  (if _bblockinghit
    (`PrimitiveComponent.AddForceAtLocation` (`self.Car_ColBox`) (* (- 1.0 (`KismetMathLibrary.NormalizeToRange` _distance 0.0 60.0)) (`KismetMathLibrary.GetDirectionUnitVector` _traceend _tracestart) 100000.0) (`SceneComponent.K2_GetComponentLocation` (`local.WheelComp`)) "None"))
  (`PrimitiveComponent.AddForceAtLocation` _car_colbox (+ (* (`SceneComponent.GetForwardVector` _car_colbox) 2500.0 (`self.AccelerationInput`) (`PrimitiveComponent.GetMass` _car_colbox)) (`KismetMathLibrary.SelectVector` (0.0 0.0 0.0) (0.0 0.0 -20000.0) (`self.isOnGround`))) (`SceneComponent.K2_GetComponentLocation` (`local.WheelComp`)) "None")
  (`PrimitiveComponent.SetCenterOfMass` (`self.Car_ColBox`) (* (25.0 0.0 0.0) (`self.AccelerationInput`)) "None")
  (`SceneComponent.K2_SetRelativeLocation` _returnvalue_2 (`KismetMathLibrary.MakeVector` 0.0 0.0 (`KismetMathLibrary.FInterpTo` _relativelocation_z (+ (* _distance -1.0) 22.0) (`GameplayStatics.GetWorldDeltaSeconds`) 2.0)) false false))

(fn `UserConstructionScript`
  (set `self.AIControllerClass` "/Game/Blueprints/Interface/AIC_VehicleAI.AIC_VehicleAI_C"))