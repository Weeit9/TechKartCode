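; Suspension component that computes a spring-damper force for a wheel through the SpringCompression event.
; Compression is the height difference between WheelPosition and GroundLocation when grounded, otherwise zero, with a per-frame debug print while grounded.
; Its change over delta time drives damping, five times stronger when not compressing.
; The event only stores SuspensionForce and previous compression; RestLength and Target inputs are unused.
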(event `Spring Compression`
  (params (SpringK :type "Float (double-precision)") (DampingC :type "Float (double-precision)") (`Rest Length` :type "Float (double-precision)") (Target :type "PrimitiveComponent Object Reference") (`Wheel Position` :type "Vector Structure") (`Ground Location` :type "Vector Structure") (`On Ground` :type Boolean))
  (bind _returnvalue (`GameplayStatics.GetWorldDeltaSeconds`))
  (bind _returnvalue_2 (- `Wheel Position_Z` `Ground Location_Z`))
  (bind _returnvalue_3 (* SpringK (`self.CurrentCompression`)))
  (if `On Ground`
    (set `self.CurrentCompression` _returnvalue_2)
    (`KismetSystemLibrary.PrintString` (`KismetStringLibrary.Conv_DoubleToString` _returnvalue_2) true true (struct :`G` 0.66 :`B` 1.0 :`A` 1.0) _returnvalue)
    (else
      (set `self.CurrentCompression` 0.0)))
  (bind _output_get (set `self.CompressionVelocity` (/ (- (`self.CurrentCompression`) (`self.PrevCompression`)) _returnvalue)))
  (if (> _output_get 0.0)
    (set `self.SuspensionForce` (- _returnvalue_3 (* DampingC (`self.CompressionVelocity`))))
    (set `self.PrevCompression` (`self.CurrentCompression`))
    (else
      (set `self.SuspensionForce` (- _returnvalue_3 (* (* DampingC 5.0) (`self.CompressionVelocity`))))
      (set `self.PrevCompression` (`self.CurrentCompression`)))))