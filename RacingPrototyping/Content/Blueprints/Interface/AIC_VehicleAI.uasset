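; AI controller that drives a race vehicle along a BP_RaceSpline path, on the left or right side of the road.
; Each tick it aims at a speed-scaled look-ahead point, lowers top speed as the path angle grows, and sends steering, throttle and brake through messages.
; A looping timer reads the vehicle's overlap boxes to switch sides for overtakes, match a blocking car's speed or nudge steering.
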(event `self.ReceiveBeginPlay`
  (set `self.ControlledVehicle` (`self.K2_GetPawn`) :!label _label)
  (bind _returnvalue (`GameplayStatics.GetActorOfClass` "/Game/Blueprints/Spline/BP_RaceSpline.BP_RaceSpline_C"))
  (set `self.AIPath` _returnvalue)
  (bind _sideofroad (`self.CalculateStartingSideOfRoad`))
  (set `self.SideOfRoad` _sideofroad)
  (`KismetSystemLibrary.K2_SetTimer` null "CheckForOvertakes" 0.1 true))

(event `self.ReceiveTick`
  (params (DeltaSeconds :type "Float (single-precision)"))
  (bind _controlledvehicle (`self.ControlledVehicle`))
  (bind _controlledvehicle_2 (`self.ControlledVehicle`))
  (`/Engine/EditorBlueprintResources/StandardMacros.IsValid` _controlledvehicle
    (:`Is Valid`
      (bind _steeringinput (`self.CalculateSteering`))
      (message `/Game/Blueprints/Interface/BPI_IsVehicle.SetSteering` _controlledvehicle _steeringinput (`self.OverrideSteering`))
      (bind _topspeed (`self.CalculateTopSpeed`))
      (bind (_throttle _brake) (`self.CalculateThrottle/brake` _topspeed))
      (message `/Game/Blueprints/Interface/BPI_IsVehicle.SetThrottle` _controlledvehicle_2 _throttle)
      (message `/Game/Blueprints/Interface/BPI_IsVehicle.SetBrake` _controlledvehicle_2 _brake))
    (:`Is Not Valid`
      (goto _label))))

(fn `CalculateStartingSideOfRoad`
  (returns (SideOfRoad :type Integer))
  (locals (LeftSideDistance :type "Float (double-precision)" :default 0.0) (RightSideDIsntance :type "Float (double-precision)" :default 0.0))
  (bind _controlledvehicle (`self.ControlledVehicle`))
  (bind _returnvalue (`self.K2_GetActorLocation` (`self.ControlledVehicle`)))
  (bind _returnvalue_2 (`self.K2_GetActorLocation` _controlledvehicle))
  ; Select Side of road based on distance to each side
  (`/Engine/EditorBlueprintResources/StandardMacros.IsValid` _controlledvehicle
    (:`Is Valid`
      (bind _locationtosteerto (message `/Game/Blueprints/Interface/BPI_isAIPath.GetClosestLocationToAIPath` (`self.AIPath`) _returnvalue_2 0.0 0))
      (set `local.LeftSideDistance` (`KismetMathLibrary.Vector_Distance` _locationtosteerto _returnvalue_2))
      (bind _locationtosteerto_2 (message `/Game/Blueprints/Interface/BPI_isAIPath.GetClosestLocationToAIPath` (`self.AIPath`) _returnvalue 0.0 1))
      (set `local.RightSideDIsntance` (`KismetMathLibrary.Vector_Distance` _locationtosteerto_2 _returnvalue))
      (return (`KismetMathLibrary.Conv_BoolToInt` (> (`local.LeftSideDistance`) (`local.RightSideDIsntance`)))))))

(fn `CalculateSteering`
  (returns (SteeringInput :type "Float (double-precision)"))
  (bind _currentspeed (message `/Game/Blueprints/Interface/BPI_IsVehicle.GetCurrentSpeed` (`self.ControlledVehicle`)))
  (bind _frontlocation (message `/Game/Blueprints/Interface/BPI_IsVehicle.GetFrontOfCar` (`self.ControlledVehicle`)))
  (bind _locationtosteerto (message `/Game/Blueprints/Interface/BPI_isAIPath.GetClosestLocationToAIPath` (`self.AIPath`) _frontlocation (`KismetMathLibrary.MapRangeClamped` _currentspeed 500.0 2000.0 1000.0 3000.0) (`self.SideOfRoad`)))
  (bind (_returnvalue_roll _returnvalue_pitch _returnvalue_yaw) (`KismetMathLibrary.BreakRotator` (`KismetMathLibrary.NormalizedDeltaRotator` (`KismetMathLibrary.FindLookAtRotation` _frontlocation _locationtosteerto) (`self.K2_GetActorRotation`))))
  (return (`KismetMathLibrary.MapRangeClamped` _returnvalue_yaw -10.0 10.0 -1.0 1.0)))

(fn `CalculateThrottle`
  (returns (AIThrottle :type "Float (double-precision)"))
  (bind _controlledvehicle (`self.ControlledVehicle`))
  (bind _returnvalue (`KismetMathLibrary.Dot_VectorVector` (`SplineComponent.FindDirectionClosestToWorldLocation` (`/Game/Blueprints/Spline/BP_RaceSpline.SplineToFollow` (`self.AIPath`)) (`self.K2_GetActorLocation` _controlledvehicle) "World") (`self.GetActorForwardVector` _controlledvehicle)))
  (return (* (`KismetMathLibrary.FClamp` (`KismetMathLibrary.Abs` _returnvalue) 0.2) (`KismetMathLibrary.SignOfFloat` _returnvalue))))

(fn `CalculateThrottle/brake`
  (params (TopSpeed :type "Float (double-precision)"))
  (returns (Throttle :type "Float (double-precision)") (Brake :type "Float (double-precision)"))
  (locals (CurrentSpeed :type "Float (double-precision)" :default 0.0))
  (bind _currentspeed (message `/Game/Blueprints/Interface/BPI_IsVehicle.GetCurrentSpeed` (`self.ControlledVehicle`)))
  (bind _output_get (set `local.CurrentSpeed` _currentspeed))
  (if (>= _output_get TopSpeed)
    (return (`KismetMathLibrary.RandomFloatInRange` 0.2 0.3) 1.0)
    (else
      (return (`KismetMathLibrary.RandomFloatInRange` 0.8 1.0) 0.0))))

(fn `CalculateTopSpeed`
  (returns (TopSpeed :type "Float (double-precision)"))
  (if (`self.OverrideTopSpeed?`)
    (return (`self.OverrideTopSpeed`))
    (else
      (bind _currentspeed (message `/Game/Blueprints/Interface/BPI_IsVehicle.GetCurrentSpeed` (`self.ControlledVehicle`)))
      (bind _frontlocation (message `/Game/Blueprints/Interface/BPI_IsVehicle.GetFrontOfCar` (`self.ControlledVehicle`)))
      (bind _locationtosteerto (message `/Game/Blueprints/Interface/BPI_isAIPath.GetClosestLocationToAIPath` (`self.AIPath`) _frontlocation (`KismetMathLibrary.MapRangeClamped` _currentspeed 500.0 2000.0 3000.0 9000.0) (`self.SideOfRoad`)))
      (bind (_returnvalue_roll _returnvalue_pitch _returnvalue_yaw) (`KismetMathLibrary.BreakRotator` (`KismetMathLibrary.NormalizedDeltaRotator` (`KismetMathLibrary.FindLookAtRotation` _frontlocation _locationtosteerto) (`self.K2_GetActorRotation`))))
      (return (`KismetMathLibrary.MapRangeClamped` (`KismetMathLibrary.Abs` _returnvalue_yaw) 0.0 40.0 2000.0 1500.0)))))

(fn `CheckForOvertakes`
  (locals (`VehicleInFront?` :type Boolean) (VehicleInFront :type "Actor Object Reference") (`VehicleInLeftSide?` :type Boolean) (`VehicleInRightSide?` :type Boolean))
  (`|ExecutionSequence`
    (:`then_0`
      ; Check in front for vehicle
      (bind _frontbox (message `/Game/Blueprints/Interface/BPI_IsVehicle.GetCollisionBoxes` (`self.ControlledVehicle`)))
      (bind _overlappingactors (`PrimitiveComponent.GetOverlappingActors` _frontbox null))
      (bind _returnvalue (> (`KismetArrayLibrary.Array_Length` _overlappingactors) 0))
      (if _returnvalue
        (set `local.VehicleInFront?` _returnvalue)
        (set `local.VehicleInFront` (`|GetArrayItem` _overlappingactors))
        (else
          (set `self.OverrideTopSpeed?` false))))
    (:`then_1`
      ; Check for vehicles left and right
      (if (`local.VehicleInFront?`)
        (if (`KismetMathLibrary.Conv_IntToBool` (`self.SideOfRoad`))
          (bind (_frontbox_2 _leftsidebox) (message `/Game/Blueprints/Interface/BPI_IsVehicle.GetCollisionBoxes` (`self.ControlledVehicle`)))
          (bind _returnvalue_2 (> (`KismetArrayLibrary.Array_Length` (`PrimitiveComponent.GetOverlappingActors` _leftsidebox null)) 0))
          (if _returnvalue_2
            (set `local.VehicleInLeftSide?` _returnvalue_2)
            (set `self.OverrideSteering` -5.0)
            (else
              (set `self.OverrideTopSpeed?` false)))
          (else
            (bind (_frontbox_3 _leftsidebox_2 _rightsidebox) (message `/Game/Blueprints/Interface/BPI_IsVehicle.GetCollisionBoxes` (`self.ControlledVehicle`)))
            (bind _returnvalue_3 (> (`KismetArrayLibrary.Array_Length` (`PrimitiveComponent.GetOverlappingActors` _rightsidebox null)) 0))
            (if _returnvalue_3
              (set `local.VehicleInRightSide?` _returnvalue_3)
              (set `self.OverrideSteering` 5.0)
              (else
                (set `self.OverrideTopSpeed?` false)))))))
    (:`then_2`
      (if (and (`local.VehicleInFront?`) (or (`local.VehicleInLeftSide?`) (`local.VehicleInRightSide?`)))
        ; Slow down if there is cars in front and sides and can't over take
        (set `self.OverrideTopSpeed?` (< (`KismetMathLibrary.Vector_Distance` (`self.K2_GetActorLocation` (`self.ControlledVehicle`)) (`self.K2_GetActorLocation` (`local.VehicleInFront`))) 750.0))
        (bind _currentspeed (message `/Game/Blueprints/Interface/BPI_IsVehicle.GetCurrentSpeed` (`local.VehicleInFront`)))
        (set `self.OverrideTopSpeed` _currentspeed)
        (else
          ; overtake
          (if (`local.VehicleInFront?`)
            (set `self.OverrideTopSpeed?` true)
            (set `self.SideOfRoad` (`KismetMathLibrary.SelectInt` 0 1 (`KismetMathLibrary.Conv_IntToBool` (`self.SideOfRoad`))))
            (set `self.OverrideTopSpeed` 10000.0)
            (else
              (set `self.OverrideTopSpeed?` false))))))
    (:`then_3`
      ; AdjustSteering based on if vehicle is on side
      (if (`local.VehicleInFront?`)
        (set `self.OverrideSteering` (`KismetMathLibrary.SelectFloat` 0.5 -0.5 (`KismetMathLibrary.RandomBool`)))
        (elif (`local.VehicleInLeftSide?`)
          (set `self.OverrideSteering` 0.5)
          (elif (`local.VehicleInRightSide?`)
            (set `self.OverrideSteering` -0.5)
            (else
              (set `self.OverrideSteering` 0.0))))))))

(fn `UserConstructionScript`)