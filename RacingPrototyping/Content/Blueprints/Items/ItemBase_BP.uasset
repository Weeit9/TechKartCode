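; ItemBase_BP is an item actor that notifies a BP_CarPawn when it overlaps one, passing its ItemID to the car's Hit function.
; BeginPlay holds projectile movement setup for speed and optional homing, or zero speed when CanMove is off, but a constant branch condition keeps it from running.
; An unconnected node that would set the mesh from DataAsset also never runs.
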(event `self.ReceiveBeginPlay`
  (bind _projectilemovement (`self.ProjectileMovement`))
  (if true
    _
    (elif (`self.CanMove`)
      (set `ProjectileMovementComponent.InitialSpeed` (`KismetMathLibrary.Conv_IntToDouble` (`self.Speed`)) _projectilemovement)
      (set `ProjectileMovementComponent.bIsHomingProjectile` (`self.IsHoming`) _projectilemovement)
      (set `ProjectileMovementComponent.HomingAccelerationMagnitude` (`KismetMathLibrary.Conv_IntToDouble` (`self.HomingStrength`)) _projectilemovement)
      (else
        (set `ProjectileMovementComponent.InitialSpeed` 0.0 _projectilemovement)))))

(event `self.HitOverlap.OnComponentBeginOverlap`
  (params (OverlappedComponent :type "PrimitiveComponent Object Reference") (OtherActor :type "Actor Object Reference") (OtherComp :type "PrimitiveComponent Object Reference") (OtherBodyIndex :type Integer) (bFromSweep :type Boolean) (SweepResult :type "HitResult Structure (by ref)"))
  (bind _asbp_car_pawn (cast `/Game/Blueprints/Car/BP_CarPawn` OtherActor))
  (`/Game/Blueprints/Car/BP_CarPawn.Hit` _asbp_car_pawn (`self.ItemID`)))

(fn `UserConstructionScript`)