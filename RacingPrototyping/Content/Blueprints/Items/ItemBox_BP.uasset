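; ItemBox_BP is an item box pickup that gives an item to a BP_CarPawn that overlaps it.
; Any overlap first starts Respawn, then calls ItemGive on the other actor if it casts to BP_CarPawn.
; Respawn disables the Overlap collision and hides the Cube, then restores both after a RespawnTimer delay, so non-car actors also consume the box.
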(event `self.ReceiveActorBeginOverlap`
  (params (OtherActor :type "Actor Object Reference"))
  (`self.Respawn`)
  (bind _asbp_car_pawn (cast `/Game/Blueprints/Car/BP_CarPawn` OtherActor))
  (`/Game/Blueprints/Car/BP_CarPawn.ItemGive` _asbp_car_pawn))

(event `Respawn`
  (`PrimitiveComponent.SetCollisionEnabled` (`self.Overlap`) "NoCollision")
  (`SceneComponent.SetVisibility` (`self.Cube`) false false)
  (`KismetSystemLibrary.Delay` (`KismetMathLibrary.Conv_IntToDouble` (`self.RespawnTimer`)))
  (`PrimitiveComponent.SetCollisionEnabled` (`self.Overlap`) "QueryOnly")
  (`SceneComponent.SetVisibility` (`self.Cube`) true false))

(fn `UserConstructionScript`)