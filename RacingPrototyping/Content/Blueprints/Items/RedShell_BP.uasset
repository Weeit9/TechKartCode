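; Red shell item that races along the track and homes in on a detected kart.
; It starts at the instigator's track distance and advances along the BP_RaceSpline by a fixed step each tick, raised above the spline.
; When VehicleDetector overlaps a player or AI kart, spline movement stops and ProjectileMovement homes on that kart's collision component.
; HitOverlap calls Hit only on BP_CarPawn, then destroys the shell.
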(event `self.ReceiveBeginPlay`
  (bind _splinetofollow (`/Game/Blueprints/Spline/BP_RaceSpline.SplineToFollow` (`self.Track`)))
  (`parent.ReceiveBeginPlay`)
  (bind _returnvalue (`GameplayStatics.GetActorOfClass` "/Game/Blueprints/Spline/BP_RaceSpline.BP_RaceSpline_C"))
  (set `self.Track` _returnvalue)
  (bind _asbp_car_pawn (cast `/Game/Blueprints/Car/BP_CarPawn` (`self.GetInstigator`)))
  (bind _distancealongtrack (`/Game/Blueprints/Car/BP_CarPawn.DistanceAlongTrack` _asbp_car_pawn))
  (set `self.CurrentSplineDistance` _distancealongtrack)
  (bind (_returnvalue_x _returnvalue_y _returnvalue_z) (`KismetMathLibrary.BreakVector` (`SplineComponent.GetLocationAtDistanceAlongSpline` _splinetofollow _distancealongtrack "World")))
  (`SceneComponent.K2_SetWorldLocationAndRotation` (`self.ItemMesh`) (`KismetMathLibrary.MakeVector` _returnvalue_x _returnvalue_y (+ _returnvalue_z 50.0)) (`SplineComponent.GetRotationAtDistanceAlongSpline` _splinetofollow _distancealongtrack "World") false false))

(event `self.ReceiveTick`
  (params (DeltaSeconds :type "Float (single-precision)"))
  (`self.MoveAlongTrack`))

(event `self.HitOverlap.OnComponentBeginOverlap`
  (params (OverlappedComponent :type "PrimitiveComponent Object Reference") (OtherActor :type "Actor Object Reference") (OtherComp :type "PrimitiveComponent Object Reference") (OtherBodyIndex :type Integer) (bFromSweep :type Boolean) (SweepResult :type "HitResult Structure (by ref)"))
  (bind _asbp_car_pawn (cast `/Game/Blueprints/Car/BP_CarPawn` OtherActor))
  (`/Game/Blueprints/Car/BP_CarPawn.Hit` _asbp_car_pawn 2)
  (`self.K2_DestroyActor`))

(event `MoveAlongTrack`
  (bind _splinetofollow (`/Game/Blueprints/Spline/BP_RaceSpline.SplineToFollow` (`self.Track`)))
  (if (`self.SeesSomeone`)
    (set `ProjectileMovementComponent.HomingAccelerationMagnitude` 3000.0 (`self.ProjectileMovement`))
    (else
      (bind _output_get (set `self.CurrentSplineDistance` (+ (`self.CurrentSplineDistance`) (`self.ShellSpeed`))))
      (bind (_returnvalue_x _returnvalue_y _returnvalue_z) (`KismetMathLibrary.BreakVector` (`SplineComponent.GetLocationAtDistanceAlongSpline` _splinetofollow _output_get "World")))
      (`SceneComponent.K2_SetWorldLocationAndRotation` (`self.ItemMesh`) (`KismetMathLibrary.MakeVector` _returnvalue_x _returnvalue_y (+ _returnvalue_z 50.0)) (`SplineComponent.GetRotationAtDistanceAlongSpline` _splinetofollow _output_get "World") false false))))

(event `self.VehicleDetector.OnComponentBeginOverlap`
  (params (OverlappedComponent :type "PrimitiveComponent Object Reference") (OtherActor :type "Actor Object Reference") (OtherComp :type "PrimitiveComponent Object Reference") (OtherBodyIndex :type Integer) (bFromSweep :type Boolean) (SweepResult :type "HitResult Structure (by ref)"))
  (if (!= (`self.GetInstigator`) OverlappedComponent)
    (bind _asbp_car_pawn (cast `/Game/Blueprints/Car/BP_CarPawn` OtherActor)
      (:`then`
        (set `self.SeesSomeone` true)
        (set `ProjectileMovementComponent.HomingTargetComponent` (`/Game/Blueprints/Car/BP_CarPawn.ItemCollision` _asbp_car_pawn) (`self.ProjectileMovement`)))
      (:`CastFailed`
        (bind _asbp_kart_with_ai (cast `/Game/Blueprints/Car/BP_KartWithAI` OtherActor))
        (set `self.SeesSomeone` true)
        (set `ProjectileMovementComponent.HomingTargetComponent` (`/Game/Blueprints/Car/BP_KartWithAI.Car_ColBox` _asbp_kart_with_ai) (`self.ProjectileMovement`))))))

(fn `UserConstructionScript`
  (`parent.UserConstructionScript`))