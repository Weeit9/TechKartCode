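; Race track spline actor that lays road meshes along SplineToFollow and supplies steering targets to AI racers.
; The construction script adds spline mesh components between consecutive spline points, with the loop count derived from spline length in fixed segments rather than from point count.
; GetClosestLocationToAIPath projects the AI location onto the spline, moves ahead by a look-ahead distance, then offsets left or right according to SideOfRoad.
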(fn `GetClosestLocationToAIPath`
  (params (AILocation :type "Vector Structure") (LookAheadDistance :type "Float (double-precision)") (SideOfRoad :type Integer))
  (returns (LocationToSteerTo :type "Vector Structure"))
  (bind _returnvalue (+ (`SplineComponent.GetDistanceAlongSplineAtLocation` (`self.SplineToFollow`) AILocation "World") (`local.LookAheadDistance`)))
  (return (+ (`SplineComponent.GetLocationAtDistanceAlongSpline` (`self.SplineToFollow`) _returnvalue "World") (* (`SplineComponent.GetRightVectorAtDistanceAlongSpline` (`self.SplineToFollow`) _returnvalue "World") (`KismetMathLibrary.SelectFloat` 200.0 -200.0 (`KismetMathLibrary.Conv_IntToBool` (`local.SideOfRoad`)))))))

(fn `UserConstructionScript`
  (bind _splinetofollow (`self.SplineToFollow`))
  (for _index (range (+ (- (`KismetMathLibrary.FFloor` (/ (`SplineComponent.GetSplineLength` (`self.SplineToFollow`)) 290.0)) 2) 1))
    (bind _returnvalue (`AddComponent|NODE_AddSplineMeshComponent-0`))
    (bind (_location _tangent) (`SplineComponent.GetLocationAndTangentAtSplinePoint` _splinetofollow _index "Local"))
    (bind (_location_2 _tangent_2) (`SplineComponent.GetLocationAndTangentAtSplinePoint` _splinetofollow (+ _index 1) "Local"))
    (`SplineMeshComponent.SetStartAndEnd` _returnvalue _location _tangent _location_2 _tangent_2 true)))