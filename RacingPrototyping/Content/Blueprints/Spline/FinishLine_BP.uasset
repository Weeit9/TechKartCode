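; FinishLine_BP is the finish line actor for the spline-based car race, detecting when cars finish.
; On BeginPlay it finds the BP_RaceSpline and snaps its root to the location and rotation of the spline's first point.
; When a BP_CarPawn with a Lap of zero or more begins overlapping FinishOverlap, it prints a finish message and calls EndRace on that pawn.
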(event `self.ReceiveBeginPlay`
  (bind _returnvalue (`GameplayStatics.GetActorOfClass` "/Game/Blueprints/Spline/BP_RaceSpline.BP_RaceSpline_C"))
  (bind _splinetofollow (`/Game/Blueprints/Spline/BP_RaceSpline.SplineToFollow` _returnvalue))
  (`SceneComponent.K2_SetWorldLocationAndRotation` (`self.DefaultSceneRoot`) (`SplineComponent.GetLocationAtSplinePoint` _splinetofollow 0 "World") (`SplineComponent.GetRotationAtSplinePoint` _splinetofollow 0 "World") false false))

(event `self.FinishOverlap.OnComponentBeginOverlap`
  (params (OverlappedComponent :type "PrimitiveComponent Object Reference") (OtherActor :type "Actor Object Reference") (OtherComp :type "PrimitiveComponent Object Reference") (OtherBodyIndex :type Integer) (bFromSweep :type Boolean) (SweepResult :type "HitResult Structure (by ref)"))
  (bind _asbp_car_pawn (cast `/Game/Blueprints/Car/BP_CarPawn` OtherActor))
  (if (>= (`/Game/Blueprints/Car/BP_CarPawn.Lap#` _asbp_car_pawn) 0)
    (`KismetSystemLibrary.PrintString` "FINISHED RACE")
    (`/Game/Blueprints/Car/BP_CarPawn.EndRace` _asbp_car_pawn)))

(fn `UserConstructionScript`)