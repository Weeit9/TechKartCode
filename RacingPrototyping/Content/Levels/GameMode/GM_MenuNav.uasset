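; GM_MenuNav is the game mode for the main menu, starting its music and UI.
; On BeginPlay it caches GI_TechRacing, creates and plays the 2D menu music at the saved MusicVolume, then adds MainMenu_WID to the viewport.
; UpdateMusicVolume rescales the playing track by MasterVolume times MusicVolume from the game instance, whereas the initial volume ignores MasterVolume.
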(event `self.ReceiveBeginPlay`
  (bind _asgi_tech_racing (cast `/Game/Levels/GameInstance/GI_TechRacing` (`GameplayStatics.GetGameInstance`)))
  (set `self.GameInstance` _asgi_tech_racing)
  (bind _returnvalue (`GameplayStatics.CreateSound2D` "/Game/Assets/Sound/Placeholder/MainMenuMusic.MainMenuMusic" 1.0 1.0 0.0 null))
  (bind _output_get (set `self.MainMenuMusic` _returnvalue))
  (`AudioComponent.SetVolumeMultiplier` _output_get (`/Game/Levels/GameInstance/GI_TechRacing.MusicVolume` _asgi_tech_racing))
  (`AudioComponent.Play` _output_get 0.0)
  (bind _returnvalue_2 (`|CreateWidget` "/Game/UI/MainMenu_WID.MainMenu_WID_C"))
  (`UserWidget.AddToViewport` _returnvalue_2 0))

(event `UpdateMusicVolume`
  (bind _gameinstance (`self.GameInstance`))
  ; Update Music Volume
  (bind _mainmenumusic (`self.MainMenuMusic`)
    (:`then`
      (`AudioComponent.SetVolumeMultiplier` _mainmenumusic (* (`/Game/Levels/GameInstance/GI_TechRacing.MasterVolume` _gameinstance) (`/Game/Levels/GameInstance/GI_TechRacing.MusicVolume` _gameinstance))))
    (:`else`)))

(fn `UserConstructionScript`)