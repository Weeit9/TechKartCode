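; Test race game mode that populates a four-slot race with local players and AI karts on BeginPlay.
; It creates local players from the GameInstance player count, spawns and possesses car pawns at PlayerStarts, then fills remaining slots with AI karts.
; Spawned racers are stored in a Pawns map.
; Placement ranking by sorted race progress and its looping timer are present but disconnected, leaving CheckPlayerProgress empty.
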(event `self.ReceiveBeginPlay`
  (bind _returnvalue (`GameplayStatics.GetActorOfClass` "/Game/Blueprints/Spline/BP_RaceSpline.BP_RaceSpline_C"))
  (set `self.Track Ref` _returnvalue)
  (bind _asgi_tech_racing (cast `/Game/Levels/GameInstance/GI_TechRacing` (`GameplayStatics.GetGameInstance`)))
  (bind _playercount (`/Game/Levels/GameInstance/GI_TechRacing.PlayerCount` _asgi_tech_racing))
  (for _index (range (+ _playercount 1))
    (bind _returnvalue_2 (`GameplayStatics.CreatePlayer` _index))
    (bind _asbp_player_controller (cast `/Game/Player/BP_PlayerController` _returnvalue_2))
    (set `/Game/Player/BP_PlayerController.Player Slot` _index _asbp_player_controller)
    (`BlueprintMapLibrary.Map_Add` (`self.Pawns`) _index))
  (bind _outactors (`GameplayStatics.GetAllActorsOfClass` "/Script/Engine.PlayerStart"))
  (for (_array_element _array_index) _outactors
    (if (< (`/Game/Levels/GameInstance/GI_TechRacing.PlayerCount` _asgi_tech_racing) _array_index)
      (break)
      (else
        (bind (_returnvalue_location _returnvalue_rotation) (`KismetMathLibrary.BreakTransform` (`self.GetTransform` _array_element)))
        (bind _returnvalue_3 (`|SpawnActorFromClass` "/Game/Blueprints/Car/BP_CarPawn.BP_CarPawn_C" (`KismetMathLibrary.MakeTransform` _returnvalue_location _returnvalue_rotation) "Undefined" "MultiplyWithRoot" null _array_index null))
        (bind _returnvalue_4 (`GameplayStatics.GetPlayerController` _array_index))
        (`/Engine/EditorBlueprintResources/StandardMacros.IsValid` _returnvalue_4
          (:`Is Valid`
            (`Controller.Possess` _returnvalue_4 _returnvalue_3)
            (`BlueprintMapLibrary.Map_Add` (`self.Pawns`) _array_index _returnvalue_3))))))
  (for _index_2 (range (+ _playercount 1) 4)
    (if (not (== _playercount 3))
      (bind _outactors_2 (`GameplayStatics.GetAllActorsOfClass` "/Script/Engine.PlayerStart"))
      (bind _returnvalue_5 (`|SpawnActorFromClass` "/Game/Blueprints/Car/BP_KartWithAI.BP_KartWithAI_C" (`KismetMathLibrary.MakeTransform` (`self.K2_GetActorLocation` (`|GetArrayItem` _outactors_2 _index_2))) "Undefined" "MultiplyWithRoot" null null))
      (`BlueprintMapLibrary.Map_Add` (`self.Pawns`) (+ _index_2 _playercount) _returnvalue_5))))

(event `Check Player Progress`)

(fn `UserConstructionScript`)